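; BP_DrivingCar is a map actor for a car that drives steadily along negative Y and periodically changes to a random color.
; BeginPlay passes a nine-second loop time and a transform offset to SetLoopTime and SetNiagaraOffset, both defined outside these graphs.
; Tick moves the actor a fixed, unswept step each frame, so speed depends on frame rate.
; A Delay in Tick throttles ChangeColor to roughly once per loop.
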(event EventBeginPlay
  (Variables|Default|SetLoopTime 9.0)
  (Class|DrivingCar|SetLoopTime (Variables|Default|GetLoopTime))
  (Class|DrivingCar|SetNiagaraOffset (Math|Transform|MakeTransform "-2850.000000,-1200.000000,20.000000" "0, 0, 0" "1.000000,1.000000,1.000000")))

(event Collision|EventActorBeginOverlap
  (params (OtherActor :type Actor%20Object%20Reference)))

(event EventTick
  (params (DeltaSeconds :type Float%20%28single-precision%29))
  (Transformation|AddActorWorldOffset "0.000000,-30.000000,0.000000")
  (Utilities|FlowControl|Delay (Variables|Default|GetLoopTime))
  (Class|DrivingCar|ChangeColor (Math|Vector4|MakeVector4 (Math|Random|RandomFloatinRange 0.0 1.0) (Math|Random|RandomFloatinRange 0.0 1.0) (Math|Random|RandomFloatinRange 0.0 1.0) 1.0)))

(fn ConstructionScript)