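; Desert tile grid actor for the world map that lays out a hexagonal field of instanced mesh tiles.
; The construction script loops over NumberX columns and NumberY rows, adding one local-space instance per cell to a single InstancedStaticMesh.
; Spacing derives from Radius using flat-top hex math, with odd columns shifted half a tile along Y to interlock.
; The event graph holds only empty stub events.
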(event EventBeginPlay)

(event Collision|EventActorBeginOverlap
  (params (OtherActor :type Actor%20Object%20Reference)))

(event EventTick
  (params (DeltaSeconds :type Float%20%28single-precision%29)))

(fn ConstructionScript
  (for _index (range 1 (Variables|Default|GetNumberY))
    (for _index_2 (range 1 (Variables|Default|GetNumberX))
      (Components|InstancedStaticMesh|AddInstance (Variables|Default|GetInstancedStaticMesh) (Math|Transform|MakeTransform (Math|Vector|SelectVector (Math|Vector|MakeVector (Math|Conversions|ToFloat(Integer) (* _index_2 (* (* (Math|Float|MakeLiteralFloat (Variables|Default|GetRadius)) 2.0) 0.75))) (* (* (Math|Float|MakeLiteralFloat (Variables|Default|GetRadius)) (Math|Float|Sqrt 3.0)) _index) 0.0) (Math|Vector|MakeVector (Math|Conversions|ToFloat(Integer) (* _index_2 (* (* (Math|Float|MakeLiteralFloat (Variables|Default|GetRadius)) 2.0) 0.75))) (+ (/ (* (Math|Float|MakeLiteralFloat (Variables|Default|GetRadius)) (Math|Float|Sqrt 3.0)) 2.0) (* _index (* (Math|Float|MakeLiteralFloat (Variables|Default|GetRadius)) (Math|Float|Sqrt 3.0)))) 0.0) (== (Math|Integer|%(Integer) _index_2 2) 0))) false))))